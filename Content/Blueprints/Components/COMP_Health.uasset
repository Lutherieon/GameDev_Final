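; Health component for a pawn that tracks clamped health and provides ragdoll death and respawn at the starting location.
; At BeginPlay it fills health and records the start location, caching the skeletal mesh only for player-controlled pawns.
; UpdateHealth calls OnTerminate at zero, and AttemptToRevive calls OnRevive if respawning is allowed.
; Terminate enables mesh physics, while Revive disables it, reattaches and realigns the mesh, returns the owner to start and restores health.
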(event Custom|EventRevive
  (CallFunction|Revive))

(event EventBeginPlay
  (bind _returnvalue (Components|GetOwner))
  (Variables|Health|Data|SetCurrentHealth (Variables|Health|Data|GetMaxHealth))
  (bind _aspawn (Utilities|Casting|CastToPawn _returnvalue))
  (Variables|Default|SetStartLocation (Transformation|GetActorLocation _returnvalue))
  (bind _asplayer_controller (Utilities|Casting|CastToPlayerController (Pawn|GetController _aspawn))
    (:then
      (Variables|Default|SetAs%20Player%20Controller _asplayer_controller)
      (Variables|Default|SetMesh (Actor|GetComponentbyClass (Components|GetOwner) "/Script/Engine.SkeletalMeshComponent")))
    (:CastFailed
      (Development|PrintString "Hello"))))

(fn UpdateHealth
  (params (Amount :type Float%20%28double-precision%29))
  (bind _output_get (Variables|Health|Data|SetCurrentHealth (Math|Float|Clamp(Float) (+ Amount (Variables|Health|Data|GetCurrentHealth)) 0.0 (Variables|Health|Data|GetMaxHealth))))
  (if (<= _output_get 0.0)
    (Default|CallOnTerminate)))

(fn Revive
  (bind _returnvalue (Components|GetOwner))
  (bind _mesh (Variables|Default|GetMesh))
  (bind _rootcomponent (Variables|/Script/Engine.Actor|GetRootComponent _returnvalue))
  (bind _returnvalue_2 (Transformation|GetWorldTransform _rootcomponent))
  (Physics|SetSimulatePhysics _mesh false)
  (Collision|SetCollisionEnabled _mesh "NoCollision")
  (Transformation|AttachComponentToComponent _mesh _rootcomponent "None" "KeepRelative" "KeepRelative" "KeepRelative" true)
  (Transformation|SetWorldTransform (Variables|Default|GetMesh) (Math|Transform|MakeTransform (- (.location _returnvalue_2) "") (Math|Rotator|CombineRotators (.rotation _returnvalue_2) "0.000000,270.000000,0.000000") (.scale _returnvalue_2)) false false)
  (Transformation|SetActorLocation (Components|GetOwner) (Variables|Default|GetStartLocation) false false)
  (Variables|Health|Data|SetCurrentHealth (Variables|Health|Data|GetMaxHealth)))

(fn Terminate
  (bind _mesh (Variables|Default|GetMesh))
  (Utilities|IsValid _mesh
    (:Is%20Valid
      (Physics|SetSimulatePhysics _mesh true)
      (Collision|SetCollisionEnabled _mesh "QueryAndPhysics"))))

(fn AttempttoRevive
  (if (Variables|Default|GetbCanRespawn)
    (Default|CallOnRevive)))