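; Player controller that shows the mouse cursor and relays player input to the controlled character.
; On BeginPlay it caches the player character and adds the Enhanced Input mapping context.
; Move, interact and revive actions, plus raw mouse movement for edge scrolling, reach the character as BPI_PlayerController interface messages.
; One shared message carries either axis values or an action enum, with a bool for revive.
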(event Input|EnhancedActionEvents|EnhancedInputActionIA_Move
  (params (ActionValue :type Vector%202D%20Structure) (ElapsedSeconds :type Float%20%28double-precision%29) (TriggeredSeconds :type Float%20%28double-precision%29) (InputAction :type Input%20Action%20Object%20Reference :default "/Game/_Game/Blueprints/Player/Input/Action/IA_Move.IA_Move"))
  (bind (_x _y) (Math|Vector2D|BreakVector2D ActionValue))
  (bind _playercharacter (Variables|Default|GetPlayerCharacter))
  ;[0.15 0.15 0.15 0.5] AxisMovement
  (bind _returnvalue (Utilities|DoesObjectImplementInterface _playercharacter "/Game/_Game/Blueprints/Interface/BPI_PlayerController.BPI_PlayerController_C"))
  (if _returnvalue
    (Class|BPIPlayerController|PlayerController(Message) _playercharacter "NewEnumerator0" 0.0 (Math|Vector2D|MakeVector2D _x _y) false false)))

(event Input|EnhancedActionEvents|EnhancedInputActionIA_Interact
  (params (ActionValue :type Boolean) (ElapsedSeconds :type Float%20%28double-precision%29) (TriggeredSeconds :type Float%20%28double-precision%29) (InputAction :type Input%20Action%20Object%20Reference :default "/Game/_Game/Blueprints/Player/Input/Action/IA_Interact.IA_Interact"))
  ;[0.15 0.15 0.15 0.5] Interaction
  (Class|BPIPlayerController|PlayerController(Message) (Variables|Default|GetPlayerCharacter) "NewEnumerator1" 0.0 (Math|Vector2D|MakeVector2D 0.0 0.0) false false))

(event Input|EnhancedActionEvents|EnhancedInputActionIA_Revive
  (params (ActionValue :type Boolean) (ElapsedSeconds :type Float%20%28double-precision%29) (TriggeredSeconds :type Float%20%28double-precision%29) (InputAction :type Input%20Action%20Object%20Reference :default "/Game/_Game/Blueprints/Player/Input/Action/UI/IA_Revive.IA_Revive"))
  ;[0.15 0.15 0.15 0.5] AttempToRevive
  (Class|BPIPlayerController|PlayerController(Message) :self (Variables|Default|GetPlayerCharacter) :PlayerAction "NewEnumerator3" :True/False ActionValue))

(event EventBeginPlay
  (bind _returnvalue (PlayerController|LocalPlayerSubsystems|GetEnhancedInputLocalPlayerSubsystem))
  (Utilities|FlowControl|Sequence
    (:then_0
      ;[0.15 0.15 0.15 0.5] Show Mouse Cursor
      (Variables|Default|SetbShowMouseCursor true)
      ;[0.15 0.15 0.15 0.5] Get Player Character
      (Variables|Default|SetPlayerCharacter (Game|GetPlayerCharacter 0)))
    (:then_1
      ;[0.15 0.15 0.15 0.5] Add Mapping Input
      (Utilities|IsValid _returnvalue
        (:Is%20Valid
          (Input|AddMappingContext _returnvalue "/Game/_Game/Blueprints/Player/Input/IMC_Player.IMC_Player" 0 "(bIgnoreAllPressedKeysUntilRelease=True,bForceImmediately=False,bNotifyUserSettings=False)"))))))

(event Input|MouseEvents|MouseX
  (params (AxisValue :type Float%20%28single-precision%29))
  ;[0.15 0.15 0.15 0.5] Edge Scroll
  (Class|BPIPlayerController|PlayerController(Message) :self (Variables|Default|GetPlayerCharacter) :PlayerAction "NewEnumerator2"))

(event Input|MouseEvents|MouseY
  (params (AxisValue :type Float%20%28single-precision%29))
  ;[0.15 0.15 0.15 0.5] Edge Scroll
  (Class|BPIPlayerController|PlayerController(Message) :self (Variables|Default|GetPlayerCharacter) :PlayerAction "NewEnumerator2"))

(fn ConstructionScript)