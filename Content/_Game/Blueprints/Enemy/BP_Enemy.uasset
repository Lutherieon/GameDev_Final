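; BP_Enemy is a melee enemy that attaches to a "Crowbar" socket on BeginPlay and attacks the player.
; Attack plays a sped-up downward-swing montage, whose notify, completion and interruption all lead to the same hit logic.
; That logic signals attack end, sphere-traces a short distance forward, and deals heavy damage through COMP_Health if it hits BP_Player.
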(event Custom|Attack
  (bind _self self)
  (bind _returnvalue (Transformation|GetActorLocation _self))
  (Animation|Montage|PlayMontage (Variables|Character|GetMesh) "/Game/_Game/Characters/Enemy/Animations/StandingMeleeAttackDownward_UE_Montage.StandingMeleeAttackDownward_UE_Montage" 3.0
    (:OnCompleted
      _)
    (:OnInterrupted
      _)
    (:OnNotifyBegin
      _))
  (Default|CallOnAttackEnd)
  (bind _outhit (Collision|SphereTraceByChannel _returnvalue (+ _returnvalue (* (Transformation|GetActorForwardVector _self) 1e+02)) 3e+01 "TraceTypeQuery1" false 0 "None"))
  (Utilities|IsValid (.HitActor (Collision|BreakHitResult _outhit))
    (:Is%20Valid
      (Utilities|Casting|CastToBP_Player (.HitActor (Collision|BreakHitResult _outhit)))
      (Utilities|IsValid (Actor|GetComponentbyClass (.HitActor (Collision|BreakHitResult _outhit)) "/Game/_Game/Blueprints/Components/COMP_Health.COMP_Health_C")
        (:Is%20Valid
          (Default|UpdateHealth (Actor|GetComponentbyClass (.HitActor (Collision|BreakHitResult _outhit)) "/Game/_Game/Blueprints/Components/COMP_Health.COMP_Health_C") -1e+02))))))

(event Custom|AddWeaponToSocket
  (Transformation|AttachComponentToComponent (Variables|Character|GetMesh) 0 "Crowbar" "SnapToTarget" "SnapToTarget" "SnapToTarget" true))

(event EventBeginPlay
  (CallFunction|AddWeapontoSocket))

(fn ConstructionScript)